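; Third-person player character Blueprint that holds no active logic: Tick, OnLanded and the construction script are all empty.
; Disconnected leftover nodes sketch an impulse gadget feature, spawning BP_ImpulseGadget ahead of and below the capsule's center.
; Other orphaned test nodes print that spawn point, launch the character upward through a movement impulse, and read control and camera rotations.
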(event `self.ReceiveTick`
  (params (DeltaSeconds :type "Float (single-precision)")))

(event `Key|RightMouseButton`
  (params (Key :type "Key Structure")))

(event `self.OnLanded`
  (params (Hit :type "HitResult Structure (by ref)")))

(fn `UserConstructionScript`)